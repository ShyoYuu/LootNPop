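; Generated dynamic mesh actor that builds one noise-displaced octant of a spherical terrain and can save it as a Nanite static mesh with complex-as-simple collision.
; On rebuild, it deletes three faces of a subdivided box and projects the remaining vertices onto a sphere.
; Perlin displacement is masked by normalized X·Y·Z, fading to zero at the octant's seam edges.
; Post-processing then welds edges, rebuilds and flips normals, and cleans up geometry.
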(event EventBeginPlay)

(event Collision|EventActorBeginOverlap
  (params (OtherActor :type Actor%20Object%20Reference)))

(event EventTick
  (params (DeltaSeconds :type Float%20%28single-precision%29)))

(event Events|EventOnRebuildGeneratedMesh
  (params (TargetMesh :type Dynamic%20Mesh%20Object%20Reference))
  (bind _output (CallFunction|CreateOctantPrimitive TargetMesh))
  (bind _output_2 (CallFunction|ApplySeamAwarePerlinNoise _output))
  (CallFunction|PostProcessTerrainGeometry _output_2))

(event EventSaveMesh
  (bind _returnvalue (DynamicMeshComponent|GetDynamicMesh (Variables|Default|GetDynamicMeshComponent)))
  (GeometryScript|AssetManagement|CreateNewStaticMeshAssetfromMesh _returnvalue (Variables|Default|GetAssetPathAndName) (Utilities|Struct|MakeGeometryScriptCreateNewStaticMeshAssetOptions false false true "(bEnabled=False,bExplicitTangents=False,bLerpUVs=True,bSeparable=False,bVoxelNDF=True,bVoxelOpacity=False,ShapePreservation=None,PositionPrecision=-2147483648,NormalPrecision=-1,TangentPrecision=-1,BoneWeightPrecision=-1,TargetMinimumResidencyInKB=0,KeepPercentTriangles=1.000000,TrimRelativeError=0.000000,GenerateFallback=PlatformDefault,FallbackTarget=Auto,FallbackPercentTriangles=1.000000,FallbackRelativeError=1.000000,MaxEdgeLengthFactor=0.000000,NumRays=64,VoxelLevel=0,RayBackUp=0.000000,DisplacementUVChannel=0,DisplacementMaps=,NaniteAssemblyData=(Parts=,Nodes=))" 0.0 true "CTF_UseComplexAsSimple")))

(fn ConstructionScript)

(fn CreateOctantPrimitive
  (params (Input :type Dynamic%20Mesh%20Object%20Reference))
  (bind _radius (Variables|Default|GetRadius))
  (bind _subdivisions (Variables|Default|GetSubdivisions))
  (bind _radius_2 (Variables|Default|GetRadius))
  (bind _returnvalue (Math|Float|SafeDivide _radius_2 2.0))
  (bind _returnvalue_2 (DynamicMesh|Reset Input))
  (bind _returnvalue_3 (Class|GeometryScriptLibraryMeshPrimitiveFunctions|AppendBox :TargetMesh _returnvalue_2 :Transform (Math|Transform|MakeTransform (Math|Vector|MakeVector _returnvalue _returnvalue _returnvalue)) :DimensionX _radius :DimensionY _radius :DimensionZ _radius :StepsX _subdivisions :StepsY _subdivisions :StepsZ _subdivisions :Origin "Center"))
  (bind (_selection _returnvalue_4) (Class|GeometryScriptLibraryMeshSelectionFunctions|SelectMeshElementsbyNormalAngle _returnvalue_3 "-1.000000,0.000000,0.000000" 1.0 "Triangles" false))
  (bind (_selection_2 _returnvalue_5) (Class|GeometryScriptLibraryMeshSelectionFunctions|SelectMeshElementsbyNormalAngle _returnvalue_4 "0.000000,-1.000000,0.000000" 1.0 "Triangles" false))
  (bind (_selection_3 _returnvalue_6) (Class|GeometryScriptLibraryMeshSelectionFunctions|SelectMeshElementsbyNormalAngle _returnvalue_5 "0.000000,0.000000,-1.000000" 1.0 "Triangles" false))
  (bind _resultselection (Class|GeometryScriptLibraryMeshSelectionFunctions|CombineMeshSelections _selection_2 _selection_3 "Add"))
  (bind _resultselection_2 (Class|GeometryScriptLibraryMeshSelectionFunctions|CombineMeshSelections _selection _resultselection "Add"))
  (bind _returnvalue_7 (Class|GeometryScriptLibraryMeshBasicEditFunctions|DeleteSelectedTrianglesfromMesh _returnvalue_6 _resultselection_2 false))
  (bind _returnvalue_8 (Class|GeometryScriptLibraryMeshRepairFunctions|CompactMesh _returnvalue_7))
  (bind (_positionlist _bhasvertexidgaps _returnvalue_9) (GeometryScript|MeshQueries|GetAllVertexPositions _returnvalue_8 true))
  (Class|GeometryScriptLibraryVectorMathFunctions|VectorNormalizeinPlace _positionlist "0, 0, 0")
  (Class|GeometryScriptLibraryVectorMathFunctions|ConstantVectorMultiplyinPlace (Variables|Default|GetRadius) _positionlist)
  (bind _returnvalue_10 (Class|GeometryScriptLibraryMeshBasicEditFunctions|SetAllMeshVertexPositions _returnvalue_9 _positionlist))
  (return _returnvalue_10))

(fn ApplySeamAwarePerlinNoise
  (params (Input :type Dynamic%20Mesh%20Object%20Reference))
  (bind _radius (Variables|Default|GetRadius))
  (bind _returnvalue (Math|Float|SafeDivide 1.0 _radius))
  ;[0.15 0.15 0.15 0.5] OriginalPos
  (bind (_positionlist _bhasvertexidgaps _returnvalue_2) (GeometryScript|MeshQueries|GetAllVertexPositions Input))
  ;[0.15 0.15 0.15 0.5] WeightMask
  (bind _returnvalue_3 (Class|GeometryScriptLibraryVectorMathFunctions|VectortoScalar _positionlist _returnvalue 0.0 0.0))
  (bind _returnvalue_4 (Class|GeometryScriptLibraryVectorMathFunctions|VectortoScalar _positionlist 0.0 _returnvalue 0.0))
  (bind _returnvalue_5 (Class|GeometryScriptLibraryVectorMathFunctions|VectortoScalar _positionlist 0.0 0.0 _returnvalue))
  (bind _returnvalue_6 (Class|GeometryScriptLibraryVectorMathFunctions|ScalarMultiply _returnvalue_3 _returnvalue_4 1.0))
  (bind _returnvalue_7 (Class|GeometryScriptLibraryVectorMathFunctions|ScalarMultiply _returnvalue_6 _returnvalue_5 1.0))
  ;[0.15 0.15 0.15 0.5] PerlinNoise
  (bind _returnvalue_8 (Class|GeometryScriptLibraryMeshDeformFunctions|ApplyPerlinNoisetoMesh2 :TargetMesh _returnvalue_2 :Options (Utilities|Struct|MakeGeometryScriptPerlinNoiseOptions (Utilities|Struct|MakeGeometryScriptPerlinNoiseLayerOptions (Variables|Default|GetMagnitude) (Variables|Default|GetFrequency) "0.000000,0.000000,0.000000" (Variables|Default|GetRandom%20Seed)) true "Computed" "FullMeshSelection")))
  ;[0.15 0.15 0.15 0.5] NoisyPos
  (bind (_positionlist_2 _bhasvertexidgaps_2 _returnvalue_9) (GeometryScript|MeshQueries|GetAllVertexPositions _returnvalue_8))
  ;[0.15 0.15 0.15 0.5] MaskedDisplacement
  (bind _returnvalue_10 (Class|GeometryScriptLibraryVectorMathFunctions|VectorBlend _positionlist_2 _positionlist 1.0 -1.0))
  (bind _returnvalue_11 (Class|GeometryScriptLibraryVectorMathFunctions|ScalarVectorMultiply _returnvalue_7 _returnvalue_10 1.0))
  ;[0.15 0.15 0.15 0.5] FinalPos
  (bind _returnvalue_12 (Class|GeometryScriptLibraryVectorMathFunctions|VectorBlend _returnvalue_11 _positionlist 1.0 1.0))
  (bind _returnvalue_13 (Class|GeometryScriptLibraryMeshBasicEditFunctions|SetAllMeshVertexPositions _returnvalue_9 _returnvalue_12))
  (return _returnvalue_13))

(fn PostProcessTerrainGeometry
  (params (Input :type Dynamic%20Mesh%20Object%20Reference))
  (bind _returnvalue (Class|GeometryScriptLibraryMeshRepairFunctions|WeldMeshEdges Input))
  (bind _returnvalue_2 (Class|GeometryScriptLibraryMeshNormalsFunctions|SetPerVertexNormals _returnvalue))
  (bind _returnvalue_3 (Class|GeometryScriptLibraryMeshNormalsFunctions|ComputeTangents _returnvalue_2))
  (bind _returnvalue_4 (GeometryScript|Normals|RecomputeNormals _returnvalue_3))
  (bind _returnvalue_5 (Class|GeometryScriptLibraryMeshNormalsFunctions|FlipNormals _returnvalue_4))
  (bind _returnvalue_6 (Class|GeometryScriptLibraryMeshRepairFunctions|RepairMeshDegenerateGeometry _returnvalue_5 (Utilities|Struct|MakeGeometryScriptDegenerateTriangleOptions "RepairOrDelete" 0.001 0.0001 true)))
  (bind _returnvalue_7 (Class|GeometryScriptLibraryMeshRepairFunctions|CompactMesh _returnvalue_6))
  (return _returnvalue_7))